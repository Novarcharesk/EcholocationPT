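; BP_Collectible is a pickup that adds to the player's collectible count when touched.
; Its Box component's overlap event accepts only player pawn 0, cast to BP_ThirdPersonCharacter, and increments that character's CollectibleCount directly.
; It then plays a 2D collect sound, spawns a collect effect at its own location and destroys itself.
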(event `self.Box.OnComponentBeginOverlap`
  (params (OverlappedComponent :type "PrimitiveComponent Object Reference") (OtherActor :type "Actor Object Reference") (OtherComp :type "PrimitiveComponent Object Reference") (OtherBodyIndex :type Integer) (bFromSweep :type Boolean) (SweepResult :type "HitResult Structure (by ref)"))
  (if (== OtherActor (`GameplayStatics.GetPlayerPawn` 0))
    (bind _asbp_third_person_character (cast `/Game/ThirdPerson/Blueprints/BP_ThirdPersonCharacter` (`GameplayStatics.GetPlayerPawn` 0)))
    (set `/Game/ThirdPerson/Blueprints/BP_ThirdPersonCharacter.Collectible Count` (+ (`/Game/ThirdPerson/Blueprints/BP_ThirdPersonCharacter.Collectible Count` _asbp_third_person_character) 1) _asbp_third_person_character)
    (`GameplayStatics.PlaySound2D` "/Game/Audio/CollectCue.CollectCue" 1.0 1.0 0.0 null null)
    (`NiagaraFunctionLibrary.SpawnSystemAtLocation` "/Game/Effects/FX_Collect.FX_Collect" (`self.K2_GetActorLocation`))
    (`self.K2_DestroyActor`)))

(fn `UserConstructionScript`)